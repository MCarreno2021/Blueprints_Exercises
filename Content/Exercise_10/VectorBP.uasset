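; VectorBP is an actor Blueprint that endlessly wanders between random destinations at a fixed height, using manual vector math.
; SetRandomDestination picks a random X/Y point on BeginPlay and again whenever the remaining distance drops below Speed.
; Each Tick normalizes the vector to the destination, scales it by Speed and delta time, and applies it as an unswept local offset, although the direction is computed in world space.
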(event `self.ReceiveBeginPlay`
  (`self.SetRandomDestination`))

(event `self.ReceiveTick`
  (params (DeltaSeconds :type "Float (single-precision)"))
  (set `self.DeltaSeconds` DeltaSeconds)
  (bind _output_get (set `self.vDistance` (- (`self.vDestination`) (`self.K2_GetActorLocation`))))
  (bind _output_get_2 (set `self.vDirection` (`KismetMathLibrary.Normal` _output_get)))
  (bind _output_get_3 (set `self.vVelocity` (* _output_get_2 (`self.Speed`))))
  (bind _output_get_4 (set `self.vStep` (* _output_get_3 (`self.DeltaSeconds`))))
  (`self.K2_AddActorLocalOffset` _output_get_4)
  (if (< (`KismetMathLibrary.VSize` (`self.vDistance`)) (`self.Speed`))
    (`self.SetRandomDestination`)))

(fn `UserConstructionScript`)